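; BP_Door is a door that swings open and closed when interacted with through InteractwithBuild.
; A timeline adds its yaw to the MainPivot rotation saved at BeginPlay, playing forward to open and in reverse to close, with IsOpening blocking input mid-swing.
; An overlap event drives a second timeline whose Lerp endpoints are both zero, so it only zeroes relative rotation.
; ReturnBoxes and GetGroupId are stubs.
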(event EventBeginPlay
  ;[1 1 1] Begin play
  (Variables|Default|SetStartPoint (Transformation|GetWorldTransform (Variables|Default|GetMainPivot))))

(event Collision|EventActorBeginOverlap
  (params (OtherActor :type Actor%20Object%20Reference))
  ;[1 1 1] Open the door
  (bind _newtrack_3 (Timeline|Timeline_0 PlayFromStart)
    (:Update
      (Transformation|SetRelativeRotation (Variables|Default|GetMainPivot) (Math|Rotator|MakeRotator 0.0 0.0 (Math|Float|Lerp 0.0 0.0 _newtrack_3)) false false))))

(event EventInteractwithBuild
  ;[1 1 1] Interact
  (if (not (Variables|Default|GetIsOpening))
    (if (not (Variables|Default|GetIsOpen))
      (Variables|Default|SetIsOpen true)
      (bind _newtrack_0 (Timeline|Timeline_3 PlayFromStart)
        (:Update
          (Variables|Default|SetIsOpening true)
          (Transformation|SetWorldRotation (Variables|Default|GetMainPivot) (Math|Rotator|MakeRotator 0.0 0.0 (+ _newtrack_0 (.yaw (.rotation (Variables|Default|GetStartPoint))))) false false))
        (:Finished
          (Variables|Default|SetIsOpening false)))
      (else
        (Variables|Default|SetIsOpen false)
        (Timeline|Timeline_3 ReverseFromEnd)))))

(fn ConstructionScript)

(fn ReturnBoxes
  (return 0))

(fn GetGroupId
  (return 0))