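; BP_Foundation is a building foundation piece that extends itself down to the terrain when spawned.
; On BeginPlay it line-traces downward from four arrow components and takes the largest ground distance found.
; It then stacks added static mesh components below itself at fixed vertical intervals to cover that gap.
; It also exposes its foundation, wall and second-floor boxes, apparently for build snapping, along with a group ID.
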(event EventBeginPlay
  ;[1 1 1] Begin play
  (CallFunction|GenerateFoundationExtension))

(fn ConstructionScript)

(fn Trace
  (params (Component :type Primitive%20Component%20Object%20Reference))
  (bind _returnvalue (Transformation|GetWorldLocation Component))
  (bind (_outhit _returnvalue_2) (Collision|LineTraceByChannel _returnvalue (+ _returnvalue "0, 0,-1000.000000") "TraceTypeQuery1" false 0 "None"))
  (return (.Distance (Collision|BreakHitResult _outhit)) _returnvalue_2))

(fn CalculateDistancefromGround
  ;[1 1 1] Calculate Distance from Ground
  (for _array_element (Utilities|Array|MakeArray (Variables|Default|GetArrow1) (Variables|Default|GetArrow2) (Variables|Default|GetArrow3) (Variables|Default|GetArrow4))
    (bind (_distance _didhit) (CallFunction|Trace _array_element))
    (if (and _didhit (> _distance (LocalVariables|GetLocalDistanceToGround)))
      (LocalVariables|SetLocalDistanceToGround _distance)))
  (return (LocalVariables|GetLocalDistanceToGround)))

(fn GenerateFoundationExtension
  ;[1 1 1] Generate Foundation Extension
  (bind _distancetoground (CallFunction|CalculateDistancefromGround))
  (for _index (range 1 (+ (Math|Float|Round (/ _distancetoground 2e+02)) 1))
    (AddComponent|AddStaticMeshComponent false (Math|Transform|MakeTransform (* "0, 0,-200.000000" _index) "0, 0, 0" "1,1,1"))))

(fn ReturnBoxes
  ;[1 1 1] Return boxes
  (return (Utilities|Array|MakeArray (Variables|Default|GetFoundation1) (Variables|Default|GetFoundation2) (Variables|Default|GetFoundation3) (Variables|Default|GetFoundation4) (Variables|Default|GetWall1) (Variables|Default|GetWall2) (Variables|Default|GetWall3) (Variables|Default|GetWall4) (Variables|Default|Get2ndFloor))))

(fn GetGroupId
  (return 0))