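; BP_Door is an interactable door for a building system that toggles open and closed through InteractwithBuild.
; It caches the Arrow component's world transform at BeginPlay and uses the Arrow as the swing pivot.
; A timeline, played forward or in reverse, adds a yaw offset to that starting rotation, while IsOpening blocks input during the motion.
; ReturnBoxes returns nothing and GetGroupId returns zero.
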(event EventBeginPlay
  ;[1 1 1] Begin play
  (Variables|Default|SetStartPoint (Transformation|GetWorldTransform (Variables|Default|GetArrow))))

(event EventInteractwithBuild
  ;[1 1 1] Interact
  (if (not (Variables|Default|GetIsOpening))
    (if (not (Variables|Default|GetIsOpen))
      (Variables|Default|SetIsOpen true)
      (bind _newtrack_0 (Timeline|Timeline_0 PlayFromStart)
        (:Update
          (Variables|Default|SetIsOpening true)
          (Transformation|SetWorldRotation (Variables|Default|GetArrow) (Math|Rotator|MakeRotator 0.0 0.0 (+ _newtrack_0 (.yaw (.rotation (Variables|Default|GetStartPoint))))) false false))
        (:Finished
          (Variables|Default|SetIsOpening false)))
      (else
        (Variables|Default|SetIsOpen false)
        (Timeline|Timeline_0 ReverseFromEnd)))))

(fn ConstructionScript)

(fn ReturnBoxes
  (return 0))

(fn GetGroupId
  ;[1 1 1] Group ID
  (return 0))