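; BP_Wood_Floor is an exterior-house actor that exposes a fixed set of boxes covering floors, walls and a second floor.
; ReturnBoxes hands back those components as one array, and GetGroupId tags the set as group zero.
; The event graph and construction script are empty, so the Blueprint only supplies data to whatever queries it.
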(event EventBeginPlay)

(event Collision|EventActorBeginOverlap
  (params (OtherActor :type Actor%20Object%20Reference)))

(event EventTick
  (params (DeltaSeconds :type Float%20%28single-precision%29)))

(fn ConstructionScript)

(fn ReturnBoxes
  ;[1 1 1] Return boxes
  (return (Utilities|Array|MakeArray (Variables|Default|GetFloor1) (Variables|Default|GetFloor2) (Variables|Default|GetFloor3) (Variables|Default|GetFloor4) (Variables|Default|GetWall1) (Variables|Default|GetWall2) (Variables|Default|GetWall3) (Variables|Default|GetWall4) (Variables|Default|Get2ndFloor))))

(fn GetGroupId
  (return 0))