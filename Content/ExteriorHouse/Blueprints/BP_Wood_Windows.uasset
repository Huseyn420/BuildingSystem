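; Interactable double wooden window for the exterior house that swings open and closed when it receives InteractwithBuild.
; BeginPlay caches both meshes' world rotations, then a timeline drives their yaw in opposite directions from those defaults, playing forward to open and reversing to close.
; An IsOpening flag ignores interaction while the animation runs.
; ReturnBoxes and GetGroupId are stubs, returning nothing and zero.
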(event EventBeginPlay
  ;[1 1 1] Begin play
  (Variables|Rotations|SetDefaultRotations (Utilities|Array|MakeArray (Transformation|GetWorldRotation (Variables|Default|GetStaticMesh_1)) (Transformation|GetWorldRotation (Variables|Default|GetStaticMesh_2)))))

(event EventInteractwithBuild
  ;[1 1 1] Interact
  (if (not (Variables|Default|GetIsOpening))
    (if (not (Variables|Default|GetIsOpen))
      (Variables|Default|SetIsOpen true)
      (bind _newtrack_0 (Timeline|Timeline_0 PlayFromStart)
        (:Update
          (Variables|Default|SetIsOpening true)
          (Transformation|SetWorldRotation (Variables|Default|GetStaticMesh_1) (Math|Rotator|MakeRotator 0.0 0.0 (+ _newtrack_0 (.yaw (Utilities|Array|Get(acopy) (Variables|Rotations|GetDefaultRotations))))) false false)
          (Transformation|SetWorldRotation (Variables|Default|GetStaticMesh_2) (Math|Rotator|MakeRotator 0.0 0.0 (+ (* _newtrack_0 -1.0) (.yaw (Utilities|Array|Get(acopy) (Variables|Rotations|GetDefaultRotations) 1)))) false false))
        (:Finished
          (Variables|Default|SetIsOpening false)))
      (else
        (Variables|Default|SetIsOpen false)
        (Timeline|Timeline_0 ReverseFromEnd)))))

(fn ConstructionScript)

(fn ReturnBoxes
  (return 0))

(fn GetGroupId
  (return 0))